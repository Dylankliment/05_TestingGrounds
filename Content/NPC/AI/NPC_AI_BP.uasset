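; AI controller for NPCs that starts the Patrol behavior tree on the PatrolData blackboard at BeginPlay.
; Perception updates only write the pawn, sensed actor and sense class to the log.
; FindPatrolRoute, not called within this file, casts the pawn to PatrollingGaurd and stores its first patrol point in the Waypoint blackboard key.
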(event OnTargetPerceptionUpdated(AIPerception)
  (params (Actor :type Actor%20Object%20Reference) (Stimulus :type AI%20Stimulus%20Structure))
  (bind _returnvalue (Class|AIPerceptionSystem|GetSenseClassforStimulus Stimulus))
  (Development|PrintString (Utilities|String|Append (Utilities|GetObjectName (Pawn|GetControlledPawn)) " " (Utilities|GetObjectName Actor) " " (Utilities|GetClassDisplayName _returnvalue)) false))

(event EventBeginPlay
  (Class|AIController|UseBlackboard "/Game/NPC/AI/PatrolData.PatrolData")
  (AI|RunBehaviorTree "/Game/NPC/AI/Patrol.Patrol"))

(event EventTick
  (params (DeltaSeconds :type Float%20%28single-precision%29)))

(fn ConstructionScript)

(fn FindPatrolRoute
  (params (Blackboard :type Blackboard%20Component%20Object%20Reference))
  (bind _aspatrolling_gaurd (Utilities|Casting|CastToPatrollingGaurd (Pawn|GetControlledPawn)))
  (AI|Components|Blackboard|SetValueasObject Blackboard (Utilities|Name|MakeLiteralName "Waypoint") (Utilities|Array|Get(acopy) (Variables|/Game/Trash/PatrollingGaurd.PatrollingGaurd_C|GetPatrol%20Points _aspatrolling_gaurd))))